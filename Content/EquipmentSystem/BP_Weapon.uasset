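; BP_Weapon is an interactable weapon actor in the world, with its static mesh set from an item data table row at construction.
; Player-tagged overlaps add or remove it from the player character's interactables: begin is bound on InteractWidget, end on InteractRange.
; Interaction events toggle the InteractWidget prompt, which rotates toward the player camera every tick.
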(event OnComponentBeginOverlap(InteractWidget)
  (params (OverlappedComponent :type Primitive%20Component%20Object%20Reference) (OtherActor :type Actor%20Object%20Reference) (OtherComp :type Primitive%20Component%20Object%20Reference) (OtherBodyIndex :type Integer) (bFromSweep :type Boolean) (SweepResult :type Hit%20Result%20Structure%20%28by%20ref%29))
  (if (Actor|ActorHasTag OtherActor (Variables|EquipmentSystem|GetPlayerTag))
    (Default|AddtoCurrentInteractables (Variables|EssentialVariable|GetPlayer%20Character) self)))

(event OnComponentEndOverlap(InteractRange)
  (params (OverlappedComponent :type Primitive%20Component%20Object%20Reference) (OtherActor :type Actor%20Object%20Reference) (OtherComp :type Primitive%20Component%20Object%20Reference) (OtherBodyIndex :type Integer))
  (if (Actor|ActorHasTag OtherActor (Variables|EquipmentSystem|GetPlayerTag))
    (Default|RemovefromCurrentInteractables (Variables|EssentialVariable|GetPlayer%20Character) self)))

(event Custom|CanBeInteractedWith
  (Rendering|SetVisibility (Variables|Default|GetInteract%20Widget) true false))

(event Custom|CantBeInteractedWith
  (Rendering|SetVisibility (Variables|Default|GetInteract%20Widget) false false))

(event EventTick
  (params (DeltaSeconds :type Float%20%28single-precision%29))
  (Transformation|SetWorldRotation (Variables|Default|GetInteract%20Widget) (UI|FaceCameraRotation) false false))

(event EventBeginPlay
  (EssentialVariable|StorePlayerCharacter))

(fn ConstructionScript
  (bind _itemdata (Variables|EquipmentSystem|GetItemData))
  (bind _returnvalue (Utilities|GetDataTableRow (.datatable (.item _itemdata)) (.rowname (.item _itemdata)))
    (:then
      (Components|StaticMesh|SetStaticMesh (Variables|Default|GetStaticMesh) (.StaticMesh (Utilities|Struct|BreakStruct_Weapons _returnvalue))))))

(fn FaceCameraRotation
  (return (Math|Rotator|FindLookatRotation (Transformation|GetWorldLocation (Variables|Default|GetInteract%20Widget)) (Transformation|GetWorldLocation (Variables|/Script/Engine.PlayerCameraManager|GetTransformComponent (Game|GetPlayerCameraManager 0))))))

(fn StorePlayerCharacter
  (bind _asbp_third_person_character (Utilities|Casting|CastToBP_ThirdPersonCharacter (Game|GetPlayerCharacter 0)))
  (Variables|EssentialVariable|SetPlayer%20Character _asbp_third_person_character))