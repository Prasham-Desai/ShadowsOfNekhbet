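; Player combat component that runs a four-attack melee combo for BP_ThirdPersonCharacter and handles sword hits.
; Grounded attack input plays the montage selected by AttackIndex, buffering presses made mid-attack for SwordAttackCombo to continue or end the chain.
; StartSwordTrace and StopSwordTrace control a looping timer that sphere-traces along the blade.
; Throttled hits apply per-attack damage, camera shake and blood to tagged actors, or play a clash sound on others.
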(event Custom|SwordAttack
  ;[0.15 0.1111 0 0.5] Sword Attack
  (Default|StopSprinting (Variables|EssentialVariables|GetCharacter))
  (if (Variables|Combat|GetIsAttacking)
    (Variables|Combat|SetSavedAttack true)
    (else
      (Variables|Combat|SetIsAttacking true)
      ;[0.15 0.1111 0 0.5] Attack based on attack index
      (switch int (Variables|Combat|GetAttackIndex)
        (:0
          (CallFunction|Attack1))
        (:1
          (CallFunction|Attack2))
        (:2
          (CallFunction|Atack3))
        (:3
          (CallFunction|Attack4))))))

(event Custom|SwordAttackCombo
  ;[0.15 0.1111 0 0.5] Attack Combo
  (Default|StopSprinting (Variables|EssentialVariables|GetCharacter))
  (if (Variables|Combat|GetSavedAttack)
    (Variables|Combat|SetSavedAttack false)
    ;[0.15 0.1111 0 0.5] Attack based on attack index
    (switch int (Variables|Combat|GetAttackIndex)
      (:0
        (CallFunction|Attack1))
      (:1
        (CallFunction|Attack2))
      (:2
        (CallFunction|Atack3))
      (:3
        (CallFunction|Attack4)))
    (else
      (CallFunction|StopCombo))))

(event Custom|StopCombo
  ;[0.15 0.1111 0 0.5] Stop Attack Combo
  (Variables|Combat|SetIsAttacking false)
  (Variables|Combat|SetAttackIndex 0))

(event Custom|Atack%203
  ;[0 0.09733 0.15 0.5] Kick Attack
  (Utilities|FlowControl|DoOnce false :!label _label
    (:Completed
      (Utilities|FlowControl|Delay 0.1)
      (Animation|Montage|PlayMontage (Variables|EssentialVariables|GetCharcterMesh) "/Game/Animations/Combat/AM_Attack_3.AM_Attack_3"
        (:then
          (Variables|Combat|SetAttackIndex 3)
          (goto _label Reset))))))

(event Custom|Attack%201
  ;[0 0.09733 0.15 0.5] First Attack
  (Utilities|FlowControl|DoOnce false :!label _label
    (:Completed
      (Utilities|FlowControl|Delay 0.1)
      (Animation|Montage|PlayMontage (Variables|EssentialVariables|GetCharcterMesh) "/Game/Animations/Combat/AM_Attack_1.AM_Attack_1"
        (:then
          (Variables|Combat|SetAttackIndex 1)
          (goto _label Reset))))))

(event Custom|Start%20Sword%20Trace
  ;[0.005086 0.02695 0.15 0.5] Sword Hit, Damage and Effects (Tracing)
  ;;[0 0.1451 0.15 0.5] Start Tracing
  (bind _returnvalue (Utilities|Time|SetTimerbyEvent (delegate Custom|Sword%20Trace%20Loop) 0.001 true))
  (Variables|Combat|SetSwordTraceLoop _returnvalue))

(event Custom|Attack%202
  ;[0 0.09733 0.15 0.5] Second Attack
  (Utilities|FlowControl|DoOnce false :!label _label
    (:Completed
      (Utilities|FlowControl|Delay 0.1)
      (Animation|Montage|PlayMontage (Variables|EssentialVariables|GetCharcterMesh) "/Game/Animations/Combat/AM_Attack_2.AM_Attack_2"
        (:then
          (Variables|Combat|SetAttackIndex 2)
          (goto _label Reset))))))

(event Custom|Sword%20Trace%20Loop
  (bind (_tip _end) (Combat|GetSwordEndPoints))
  ;[0.005086 0.02695 0.15 0.5] Sword Hit, Damage and Effects (Tracing)
  (bind (_outhit _returnvalue) (Collision|SphereTraceByChannel _tip _end 1e+01 "TraceTypeQuery1" false 0 "ForDuration" true "(R=1.000000,G=0.000000,B=0.000000,A=1.000000)" "(R=0.000000,G=1.000000,B=0.000000,A=1.000000)" 0.3))
  (if _returnvalue
    (Combat|SaveSwordHitVariables (.Location (Collision|BreakHitResult _outhit)) (.Normal (Collision|BreakHitResult _outhit)) (.HitActor (Collision|BreakHitResult _outhit)))
    ;;[0 0.1205 0.15 0.5] Check whether hit actor is enemy or not
    (if (Actor|ActorHasTag (Variables|Combat|GetSwordHitActor) (Variables|Combat|GetDamageableActorTag))
      ;;[0.15 0 0.01176 0.5] Enemy Sword Hit Logic
      (Utilities|FlowControl|DoOnce false :!label _label
        (:Completed
          (Combat|GetAttackDamageBasedonAttack)
          (Combat|HitEnemyDamageandEffects (Variables|Combat|GetAttackDamage))
          (Utilities|FlowControl|Delay 0.5)
          (goto _label Reset)))
      (else
        ;;[0 0.144 0.15 0.5] Non enemy sword hit logic
        (Utilities|FlowControl|DoOnce false :!label _label_2
          (:Completed
            (Audio|PlaySoundatLocation "/Game/Sounds/Player/SwordHitSounds/SW_SwordClash.SW_SwordClash" (Variables|Combat|GetSwordHitLocation) "0, 0, 0" 1.0 1.0 0.0 0 0 0 0)
            (Utilities|FlowControl|Delay 0.5)
            (goto _label_2 Reset)))))))

(event Custom|Attack%204
  ;[0 0.09733 0.15 0.5] Third Attack
  (Utilities|FlowControl|DoOnce false :!label _label
    (:Completed
      (Utilities|FlowControl|Delay 0.1)
      (Animation|Montage|PlayMontage (Variables|EssentialVariables|GetCharcterMesh) "/Game/Animations/Combat/AM_Attack_4.AM_Attack_4"
        (:then
          (Variables|Combat|SetAttackIndex 0)
          (goto _label Reset))))))

(event Custom|StopSwordTrace
  ;[0.005086 0.02695 0.15 0.5] Sword Hit, Damage and Effects (Tracing)
  ;;[0 0.1451 0.15 0.5] Stop Tracing
  (Utilities|Time|ClearandInvalidateTimerbyHandle (Variables|Combat|GetSwordTraceLoop)))

(event Input|EnhancedActionEvents|EnhancedInputActionIA_Attack
  (params (ActionValue :type Boolean) (ElapsedSeconds :type Float%20%28double-precision%29) (TriggeredSeconds :type Float%20%28double-precision%29) (InputAction :type Input%20Action%20Object%20Reference :default "/Game/Input/Actions/IA_Attack.IA_Attack"))
  ;[0.15 0.1111 0 0.5] Attack Input
  (:Started
    (if (and (Variables|Combat|GetCanAttack) (Combat|CheckifJumping))
      (CallFunction|SwordAttack))))

(event EventBeginPlay
  ;[0.000173 0.1021 0.15 0.5] Get Essential Variables
  (EssentialVariables|GetCharacterMesh))

(fn GetCharacterMesh
  (bind _asbp_third_person_character (Utilities|Casting|CastToBP_ThirdPersonCharacter (Components|GetOwner)))
  (Variables|EssentialVariables|SetCharacter _asbp_third_person_character)
  (Variables|EssentialVariables|SetCharcterMesh (Variables|/Script/Engine.Character|GetMesh _asbp_third_person_character)))

(fn GetSwordEndPoints
  (return (Transformation|GetWorldLocation (Variables|/Game/ThirdPerson/Blueprints/BP_ThirdPersonCharacter.BP_ThirdPersonCharacter_C|GetBlade%20Tip (Variables|EssentialVariables|GetCharacter))) (Transformation|GetWorldLocation (Variables|/Game/ThirdPerson/Blueprints/BP_ThirdPersonCharacter.BP_ThirdPersonCharacter_C|GetBlade%20End (Variables|EssentialVariables|GetCharacter)))))

(fn SaveSwordHitVariables
  (params (SwordHitLocation :type Vector) (SwordHitNormal :type Vector) (SwordHitActor :type Actor%20Object%20Reference))
  (Variables|Combat|SetSwordHitLocation SwordHitLocation)
  (Variables|Combat|SetSwordHitNormal SwordHitNormal)
  (Variables|Combat|SetSwordHitActor SwordHitActor))

(fn HitEnemyDamageandEffects
  (params (Attack%20Damage :type Float%20%28single-precision%29))
  (bind _swordhitnormal (Variables|Combat|GetSwordHitNormal))
  (Game|Damage|ApplyDamage (Variables|Combat|GetSwordHitActor) Attack%20Damage 0 (Variables|EssentialVariables|GetCharacter))
  (Camera|PlayWorldCameraShake "/Game/Blueprints/BP_SwordHitCameraShake.BP_SwordHitCameraShake_C" (Variables|Combat|GetSwordHitLocation) 0.0 2e+03)
  (Effects|SpawnEmitteratLocation "/Game/Realistic_Starter_VFX_Pack_Vol2/Particles/Blood/P_Blood_Splat_Cone.P_Blood_Splat_Cone" (Variables|Combat|GetSwordHitLocation) (Math|Rotator|MakeRotfromXY _swordhitnormal _swordhitnormal)))

(fn GetPlayerStats
  (return (Variables|/Game/ThirdPerson/Blueprints/BP_ThirdPersonCharacter.BP_ThirdPersonCharacter_C|GetPlayer%20Stats (Variables|EssentialVariables|GetCharacter))))

(fn GetAttackDamageBasedonAttack
  (bind _player_stats (Combat|GetPlayerStats))
  (switch int (Variables|Combat|GetAttackIndex)
    (:0
      (Variables|Combat|SetAttackDamage (Variables|/Game/Blueprints/Components/BPC_PlayerStats.BPC_PlayerStats_C|GetSwordAttack1Damage _player_stats)))
    (:1
      (Variables|Combat|SetAttackDamage (Variables|/Game/Blueprints/Components/BPC_PlayerStats.BPC_PlayerStats_C|GetSwordAttack2Damage _player_stats)))
    (:2
      (Variables|Combat|SetAttackDamage (Variables|/Game/Blueprints/Components/BPC_PlayerStats.BPC_PlayerStats_C|GetSwordAttack3Damage _player_stats)))
    (:3
      (Variables|Combat|SetAttackDamage (Variables|/Game/Blueprints/Components/BPC_PlayerStats.BPC_PlayerStats_C|GetSwordAttack4Damage _player_stats)))))

(fn CheckifJumping
  (return (not (Default|IsFalling (Variables|EssentialVariables|GetCharacter)))))