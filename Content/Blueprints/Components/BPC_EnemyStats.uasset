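; BPC_EnemyStats is a component that tracks current and maximum health for a BP_Dummy enemy.
; On BeginPlay it caches the owning dummy, whose health bar widget component supplies the WBP_EnemyHealthBar.
; Functions change or initialize health and push the resulting percentage to that bar, with damage reporting whether health reaches zero.
; Damage clamps stored health, while healing clamps only the returned value, so stored health can exceed the maximum.
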(event EventBeginPlay
  (EssentialVariables|StoreEnemyCharacter))

(fn StoreEnemyCharacter
  (bind _asbp_dummy (Utilities|Casting|CastToBP_Dummy (Components|GetOwner)))
  (Variables|EssentialVariables|SetEnemyCharacter _asbp_dummy)
  (return))

(fn CalculateDecrementedHealth
  (params (Damage%20Taken :type Float%20%28double-precision%29))
  (return (Math|Float|Clamp(Float) (- (Variables|Health|GetCurrentHealth) Damage%20Taken) 0.0 (Variables|Health|GetMaxHealth))))

(fn DecreaseHealth
  (params (Damage%20Taken :type Float%20%28double-precision%29))
  (bind _output_get (Variables|Health|SetCurrentHealth (Health|CalculateDecrementedHealth Damage%20Taken)))
  (Default|SetHealthBarPercentage (UI|GetHUDWidget) (Health|GetHealthPercentage))
  (if (<= _output_get 0.0)
    (return true)
    (else
      (return false))))

(fn IncreaseMaxHealth
  (params (MaxHealthGain :type Float%20%28double-precision%29))
  (bind _output_get (Variables|Health|SetMaxHealth (+ MaxHealthGain (Variables|Health|GetMaxHealth))))
  (Default|SetHealthBarPercentage (UI|GetHUDWidget) (Health|GetHealthPercentage))
  (return _output_get))

(fn IncreaseCurrentHealth
  (params (HealthGain :type Float%20%28double-precision%29))
  (bind _output_get (Variables|Health|SetCurrentHealth (+ HealthGain (Variables|Health|GetCurrentHealth))))
  (Default|SetHealthBarPercentage (UI|GetHUDWidget) (Health|GetHealthPercentage))
  (return (Math|Float|Clamp(Float) _output_get 0.0 (Variables|Health|GetMaxHealth))))

(fn GetHealthPercentage
  (return (Math|Float|SafeDivide (Variables|Health|GetCurrentHealth) (Variables|Health|GetMaxHealth))))

(fn GetHUDWidget
  (bind _aswbp_enemy_health_bar (Utilities|Casting|CastToWBP_EnemyHealthBar (UserInterface|GetWidget (Variables|/Game/Blueprints/Characters/BP_Dummy.BP_Dummy_C|GetHealthBarWidget (Variables|EssentialVariables|GetEnemyCharacter)))))
  (return _aswbp_enemy_health_bar))

(fn SetHealthtoMaxonStart
  (params (HUD%20Widget :type WBP%20HUD%20Object%20Reference))
  (Variables|Health|SetCurrentHealth (Variables|Health|GetMaxHealth))
  (Default|SetHealthBarPercentage HUD%20Widget (Health|GetHealthPercentage)))