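; BP_Dummy is an enemy character that the player can hit, target-lock or stealth-assassinate.
; Player damage picks a directional hit montage from the player's local-space position, adds knockback and a grunt, and reduces EnemyStats health.
; Death plays a montage, drops Pawn and Visibility collision, ragdolls on blend-out and frees target lock.
; An overlap range toggles the assassination prompt, which turns toward the camera each tick with the health bar.
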(event OnComponentBeginOverlap(AssassinationRange)
  (params (OverlappedComponent :type Primitive%20Component%20Object%20Reference) (OtherActor :type Actor%20Object%20Reference) (OtherComp :type Primitive%20Component%20Object%20Reference) (OtherBodyIndex :type Integer) (bFromSweep :type Boolean) (SweepResult :type Hit%20Result%20Structure%20%28by%20ref%29))
  ;[0 0.15 0.1361 0.5] Assassination toggle visibility
  (Utilities|Casting|CastToBP_ThirdPersonCharacter OtherActor)
  (Rendering|SetVisibility (Variables|Default|GetAssassinationWidget) true false))

(event OnComponentEndOverlap(AssassinationRange)
  (params (OverlappedComponent :type Primitive%20Component%20Object%20Reference) (OtherActor :type Actor%20Object%20Reference) (OtherComp :type Primitive%20Component%20Object%20Reference) (OtherBodyIndex :type Integer))
  ;[0 0.15 0.1361 0.5] Assassination toggle visibility
  (Utilities|Casting|CastToBP_ThirdPersonCharacter OtherActor)
  (Rendering|SetVisibility (Variables|Default|GetAssassinationWidget) false false))

(event Custom|PlayDeathAnimMontage
  (params (DeathMontage :type Anim%20Montage%20Object%20Reference))
  ;[0.15 0.006585 0 0.5] Play Death Anim and Set Ragdoll
  (Animation|Montage|PlayMontage (Variables|Character|GetMesh) DeathMontage
    (:then
      (DamageSystem|ChangeEnemyCollisionSettingsAfterDeath))
    (:OnBlendOut
      (Physics|SetSimulatePhysics (Variables|Character|GetMesh) true))))

(event Game|Damage|EventAnyDamage
  (params (Damage :type Float%20%28single-precision%29) (DamageType :type Damage%20Type%20Object%20Reference) (InstigatedBy :type Controller%20Object%20Reference) (DamageCauser :type Actor%20Object%20Reference))
  ;[0.15 0.001557 0 0.5] Apply Damage
  (Variables|DamageSystem|SetDamageReceived Damage)
  (if (== DamageCauser (Variables|EssentialVariables|GetPlayerCharacter))
    (DamageSystem|CalculateHitDirection (Variables|EssentialVariables|GetPlayerCharacter))
    (DamageSystem|GetHitAnimationandEffects)
    (bind _isenemydead (Default|DecreaseHealth (Variables|Default|GetEnemy%20Stats) (Variables|DamageSystem|GetDamageReceived)))
    (if _isenemydead
      (CallFunction|PlayDeathAnimMontage (Utilities|Array|Get(acopy) (Variables|DamageSystem|GetDeathAnimations) (Variables|DamageSystem|GetReactionIndex)))
      (if (Variables|TargetLock|GetIsPlayerLockedOnTo)
        (Default|FreeTargetLock (Variables|EssentialVariables|GetPlayerCharacter))))))

(event EventTick
  (params (DeltaSeconds :type Float%20%28single-precision%29))
  ;[0 0.15 0.0442 0.5] Set Rotation for Widget to face cameras
  (Transformation|SetWorldRotation (Variables|Default|GetAssassinationWidget) (UI|FaceCameraRotation) false false)
  (Transformation|SetWorldRotation (Variables|Default|GetHealthBarWidget) (UI|FaceCameraRotation) false false))

(event EventBeginPlay
  ;[0 0.15 0.0442 0.5] Store Essential Variables
  (EssentialVariables|StorePlayerCharacter))

(event EventTargetLockedon
  ;[0.06255 0.01131 0.15 0.5] Player Locked On To Self
  (Variables|TargetLock|SetIsPlayerLockedOnTo true))

(fn ConstructionScript)

(fn FaceCameraRotation
  (return (Math|Rotator|FindLookatRotation (Transformation|GetWorldLocation (Variables|Default|GetAssassinationWidget)) (Transformation|GetWorldLocation (Variables|/Script/Engine.PlayerCameraManager|GetTransformComponent (Game|GetPlayerCameraManager 0))))))

(fn StorePlayerCharacter
  (bind _asbp_third_person_character (Utilities|Casting|CastToBP_ThirdPersonCharacter (Game|GetPlayerCharacter 0)))
  (Variables|EssentialVariables|SetPlayerCharacter _asbp_third_person_character))

(fn CalculateHitDirection
  (params (PlayerCharacter :type Actor%20Object%20Reference))
  (bind _returnvalue (DamageSystem|GetDistanceBetweenPlayerandEnemy PlayerCharacter))
  (bind _returnvalue_2 (Transformation|GetActorTransform))
  (bind _returnvalue_3 (Math|Transform|InverseTransformDirection _returnvalue_2 _returnvalue))
  (if (> (Math|Float|Absolute(Float) (.x _returnvalue_3)) (Math|Float|Absolute(Float) (.y _returnvalue_3)))
    ;[0.15 0 0.137 0.5] Determine if its front or back ?
    (if (> (.x _returnvalue_3) 0.0)
      ;;[0.15 0.114 0 0.5] Front
      (Variables|DamageSystem|SetReactionIndex 1)
      (else
        ;;[0.15 0.114 0 0.5] Back
        (Variables|DamageSystem|SetReactionIndex 0)))
    (else
      ;[0.15 0 0.137 0.5] Determine if its left or right ?
      (if (> (.y _returnvalue_3) 0.0)
        ;;[0.15 0.114 0 0.5] Right
        (Variables|DamageSystem|SetReactionIndex 3)
        (else
          ;;[0.15 0.114 0 0.5] Left
          (Variables|DamageSystem|SetReactionIndex 2))))))

(fn CalculateLaunchVelocity
  (return (* (Math|Vector|GetForwardVector (Transformation|GetActorRotation (Variables|EssentialVariables|GetPlayerCharacter))) (Variables|DamageSystem|GetKnockbackForce))))

(fn GetDistanceBetweenPlayerandEnemy
  (params (Player :type Actor%20Object%20Reference))
  (return (- (Transformation|GetActorLocation Player) (Transformation|GetActorLocation))))

(fn ChangeEnemyCollisionSettingsAfterDeath
  (Collision|SetCollisionEnabled (Variables|Default|GetAssassination%20Range) "NoCollision")
  (Collision|SetCollisionResponsetoChannel (Variables|Default|GetAssassinationWidget) "ECC_Pawn" "ECR_Ignore")
  (Collision|SetCollisionResponsetoChannel (Variables|Default|GetAssassinationWidget) "ECC_Visibility" "ECR_Ignore")
  (Rendering|SetVisibility (Variables|Default|GetHealthBarWidget) false false)
  (return))

(fn GetHitAnimationandEffects
  (Animation|PlayAnimMontage (Utilities|Array|Get(acopy) (Variables|DamageSystem|GetHitAnimations) (Variables|DamageSystem|GetReactionIndex)) 1.0 "None")
  (Audio|PlaySoundatLocation "/Game/Sounds/Enemy/MSS_EnemyHitGrunt.MSS_EnemyHitGrunt" (Transformation|GetActorLocation) "0, 0, 0" 1.0 1.0 0.0 0 0 0 0)
  (Character|LaunchCharacter (DamageSystem|CalculateLaunchVelocity) true false))

(fn StealthBackAssassinate
  (Rendering|SetVisibility (Variables|Default|GetAssassinationWidget) true false)
  (CallFunction|PlayDeathAnimMontage "/Game/Animations/Assassinations/AM_StealthDeath.AM_StealthDeath")
  (return (Transformation|GetWorldLocation (Variables|Default|GetAssasinationRef)) (Transformation|GetActorRotation)))