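; Combat component for BP_ThirdPersonCharacter that runs a four-step melee combo of two sword attacks, a kick and a final attack.
; IA_Attack, gated by CanAttack, starts the current step or buffers a press made mid-attack.
; SwordAttackCombo, not called within this file, consumes the buffer to continue or resets the combo.
; Each DoOnce-guarded step plays a montage on the cached mesh after a short delay, then advances AttackIndex.
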(event Custom|SwordAttack
  ;[0.15 0.1111 0 0.5] Sword Attack
  (if (Variables|Combat|GetIsAttacking)
    (Variables|Combat|SetSavedAttack true)
    (else
      (Variables|Combat|SetIsAttacking true)
      (switch int (Variables|Combat|GetAttackIndex)
        (:0
          (CallFunction|Attack1))
        (:1
          (CallFunction|Attack2))
        (:2
          (CallFunction|AtackKick))
        (:3
          (CallFunction|Attack3))))))

(event Custom|SwordAttackCombo
  ;[0.15 0.1111 0 0.5] Attack Combo
  (if (Variables|Combat|GetSavedAttack)
    (Variables|Combat|SetSavedAttack false)
    (switch int (Variables|Combat|GetAttackIndex)
      (:0
        (CallFunction|Attack1))
      (:1
        (CallFunction|Attack2))
      (:2
        (CallFunction|AtackKick))
      (:3
        (CallFunction|Attack3)))
    (else
      (CallFunction|StopCombo))))

(event Custom|StopCombo
  ;[0.15 0.1111 0 0.5] Stop Attack Combo
  (Variables|Combat|SetIsAttacking false)
  (Variables|Combat|SetAttackIndex 0))

(event Custom|Atack%20Kick
  ;[0 0.09733 0.15 0.5] Kick Attack
  (Utilities|FlowControl|DoOnce false :!label _label
    (:Completed
      (Utilities|FlowControl|Delay 0.1)
      (Animation|Montage|PlayMontage (Variables|EssentialVariables|GetCharcterMesh) "/Game/Characters/RPG_Character/Animations/Combat/AM_Kick.AM_Kick"
        (:then
          (Variables|Combat|SetAttackIndex 3)
          (goto _label Reset))))))

(event Custom|Attack%201
  ;[0 0.09733 0.15 0.5] First Attack
  (Utilities|FlowControl|DoOnce false :!label _label
    (:Completed
      (Utilities|FlowControl|Delay 0.1)
      (Animation|Montage|PlayMontage (Variables|EssentialVariables|GetCharcterMesh) "/Game/Characters/RPG_Character/Animations/Combat/AM_Attack1.AM_Attack1"
        (:then
          (Variables|Combat|SetAttackIndex 1)
          (goto _label Reset))))))

(event Custom|Attack%202
  ;[0 0.09733 0.15 0.5] Second Attack
  (Utilities|FlowControl|DoOnce false :!label _label
    (:Completed
      (Utilities|FlowControl|Delay 0.1)
      (Animation|Montage|PlayMontage (Variables|EssentialVariables|GetCharcterMesh) "/Game/Characters/RPG_Character/Animations/Combat/AM_Attack2.AM_Attack2"
        (:then
          (Variables|Combat|SetAttackIndex 2)
          (goto _label Reset))))))

(event Custom|Attack%203
  ;[0 0.09733 0.15 0.5] Third Attack
  (Utilities|FlowControl|DoOnce false :!label _label
    (:Completed
      (Utilities|FlowControl|Delay 0.1)
      (Animation|Montage|PlayMontage (Variables|EssentialVariables|GetCharcterMesh) "/Game/Characters/RPG_Character/Animations/Combat/AM_Attack3.AM_Attack3"
        (:then
          (Variables|Combat|SetAttackIndex 0)
          (goto _label Reset))))))

(event Input|EnhancedActionEvents|EnhancedInputActionIA_Attack
  (params (ActionValue :type Boolean) (ElapsedSeconds :type Float%20%28double-precision%29) (TriggeredSeconds :type Float%20%28double-precision%29) (InputAction :type Input%20Action%20Object%20Reference :default "/Game/Input/Actions/IA_Attack.IA_Attack"))
  ;[0.15 0.1111 0 0.5] Attack Input
  (:Started
    (if (Variables|Combat|GetCanAttack)
      (CallFunction|SwordAttack))))

(event EventBeginPlay
  (EssentialVariables|GetCharacterMesh))

(fn GetCharacterMesh
  (bind _asbp_third_person_character (Utilities|Casting|CastToBP_ThirdPersonCharacter (Components|GetOwner)))
  (Variables|EssentialVariables|SetCharcterMesh (Variables|/Script/Engine.Character|GetMesh _asbp_third_person_character)))