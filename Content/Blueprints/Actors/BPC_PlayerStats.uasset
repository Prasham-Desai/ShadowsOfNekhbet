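; Player stats component that tracks health, stamina, XP and level, pushing changes to the HUD widget on the cached BP_ThirdPersonCharacter.
; Decreases clamp to valid ranges and return depletion status (true at zero health, false at zero stamina).
; Stamina gains clamp before storing, while health gains clamp only the returned value.
; Reaching max XP levels up with a sound, raises the threshold and recursively re-applies carryover XP.
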(event EventBeginPlay
  (EssentialVariables|StorePlayerCharacter))

(fn StorePlayerCharacter
  (bind _asbp_third_person_character (Utilities|Casting|CastToBP_ThirdPersonCharacter (Game|GetPlayerCharacter 0)))
  (Variables|EssentialVariables|SetPlayerCharacter _asbp_third_person_character)
  (return))

(fn CalculateDecrementedHealth
  (params (Damage%20Taken :type Float%20%28double-precision%29))
  (return (Math|Float|Clamp(Float) (- (Variables|Health|GetCurrentHealth) Damage%20Taken) 0.0 (Variables|Health|GetMaxHealth))))

(fn DecreaseHealth
  (params (Damage%20Taken :type Float%20%28double-precision%29))
  (bind _output_get (Variables|Health|SetCurrentHealth (Health|CalculateDecrementedHealth Damage%20Taken)))
  (Default|SetHealthBarPercentage (UI|GetHUDWidget) (Health|GetHealthPercentage))
  (if (<= _output_get 0.0)
    (return true)
    (else
      (return false))))

(fn IncreaseMaxHealth
  (params (MaxHealthGain :type Float%20%28double-precision%29))
  (bind _output_get (Variables|Health|SetMaxHealth (+ MaxHealthGain (Variables|Health|GetMaxHealth))))
  (Default|SetHealthBarPercentage (UI|GetHUDWidget) (Health|GetHealthPercentage))
  (return _output_get))

(fn IncreaseCurrentHealth
  (params (HealthGain :type Float%20%28double-precision%29))
  (bind _output_get (Variables|Health|SetCurrentHealth (+ HealthGain (Variables|Health|GetCurrentHealth))))
  (Default|SetHealthBarPercentage (UI|GetHUDWidget) (Health|GetHealthPercentage))
  (return (Math|Float|Clamp(Float) _output_get 0.0 (Variables|Health|GetMaxHealth))))

(fn CalculateDepletedStamina
  (params (StaminaDepletion :type Float%20%28double-precision%29))
  (return (Math|Float|Clamp(Float) (- (Variables|Stamina|GetCurrentStamina) StaminaDepletion) 0.0 (Variables|Stamina|GetMaxStamina))))

(fn DecreaseStamina
  (params (StaminaDepletion :type Float%20%28double-precision%29))
  (bind _output_get (Variables|Stamina|SetCurrentStamina (Stamina|CalculateDepletedStamina StaminaDepletion)))
  (Default|SetStaminaBarPercentage (UI|GetHUDWidget) (Stamina|GetStaminaPercentage))
  (if (<= _output_get 0.0)
    (return false)
    (else
      (return true))))

(fn IncreaseMaxStamina
  (params (MaxStaminaGain :type Float%20%28double-precision%29))
  (bind _output_get (Variables|Stamina|SetMaxStamina (+ MaxStaminaGain (Variables|Stamina|GetMaxStamina))))
  (Default|SetStaminaBarPercentage (UI|GetHUDWidget) (Stamina|GetStaminaPercentage))
  (return _output_get))

(fn IncreaseCurrentStamina
  (params (StaminaGain :type Float%20%28double-precision%29))
  (bind _output_get (Variables|Stamina|SetCurrentStamina (Math|Float|Clamp(Float) (+ StaminaGain (Variables|Stamina|GetCurrentStamina)) 0.0 (Variables|Stamina|GetMaxStamina))))
  (Default|SetStaminaBarPercentage (UI|GetHUDWidget) (Stamina|GetStaminaPercentage))
  (return _output_get))

(fn GetHealthPercentage
  (return (Math|Float|SafeDivide (Variables|Health|GetCurrentHealth) (Variables|Health|GetMaxHealth))))

(fn GetHUDWidget
  (return (Variables|/Game/ThirdPerson/Blueprints/BP_ThirdPersonCharacter.BP_ThirdPersonCharacter_C|GetHUD%20Widget (Variables|EssentialVariables|GetPlayerCharacter))))

(fn SetHealthtoMaxonStart
  (params (HUD%20Widget :type WBP%20HUD%20Object%20Reference))
  (Variables|Health|SetCurrentHealth (Variables|Health|GetMaxHealth))
  (Default|SetHealthBarPercentage HUD%20Widget (Health|GetHealthPercentage)))

(fn SetStaminatoMaxonStart
  (params (HUD%20Widget :type WBP%20HUD%20Object%20Reference))
  (Variables|Stamina|SetCurrentStamina (Variables|Stamina|GetMaxStamina))
  (Default|SetStaminaBarPercentage HUD%20Widget (Stamina|GetStaminaPercentage)))

(fn GetStaminaPercentage
  (return (Math|Float|SafeDivide (Variables|Stamina|GetCurrentStamina) (Variables|Stamina|GetMaxStamina))))

(fn IncreaseXP
  (params (Added%20XP :type Integer))
  (Variables|Level&XP|SetXP (+ Added%20XP (Variables|Level&XP|GetXP)))
  (Default|SetXPBarPercentage (UI|GetHUDWidget) (Level&XP|GetXPPercentage))
  (if (>= (Variables|Level&XP|GetXP) (Variables|Level&XP|GetMaxXP))
    (Level&XP|IncreaseLevel (Level&XP|CalculateCarryoverXP))
    (Default|SetXPText (UI|GetHUDWidget) (Level&XP|GetXPText))))

(fn IncreaseLevel
  (params (CarryOver%20XP :type Integer))
  (bind _result (Math|Integer|IncrementInt (Variables|Level&XP|GetLevel))
    (:%20%20
      (Audio|PlaySound2D "/Game/Sounds/Player/SW_LevelUp.SW_LevelUp" 1.0 1.0 0.0 0 0)
      (Default|SetLevelText (UI|GetHUDWidget) (Utilities|Text|ToText(Integer) _result))
      (Variables|Level&XP|SetXP 0)
      (Variables|Level&XP|SetMaxXP (Level&XP|CalculateIncreasedMaxXP))
      (Level&XP|IncreaseXP CarryOver%20XP))))

(fn CalculateCarryoverXP
  (return (- (Variables|Level&XP|GetXP) (Variables|Level&XP|GetMaxXP))))

(fn CalculateIncreasedMaxXP
  (return (+ (Variables|Level&XP|GetMaxXP) (Variables|Level&XP|GetMaxXPIncreasePerLvl))))

(fn GetXPPercentage
  (return (/ (Math|Conversions|ToFloat(Integer) (Variables|Level&XP|GetXP)) (Math|Conversions|ToFloat(Integer) (Variables|Level&XP|GetMaxXP)))))

(fn GetXPText
  (return (Utilities|Text|FormatText "{Current XP} / {Max XP}" (Variables|Level&XP|GetXP) (Variables|Level&XP|GetMaxXP))))