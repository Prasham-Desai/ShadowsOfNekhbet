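; BP_PlayerStats is an actor that stores and manages the player's health and stamina.
; On BeginPlay it sets both current values to their maximums.
; Decrease functions subtract through clamped helpers, with DecreaseHealth returning true once health is depleted and DecreaseStamina returning true while stamina remains.
; Increase functions raise and return the maximums without changing current values.
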(event EventBeginPlay
  (Health|SetCurrentHealthtoMaxStart)
  (Stamina|SetCurrentStaminatoMaxonStart))

(event Collision|EventActorBeginOverlap
  (params (OtherActor :type Actor%20Object%20Reference)))

(event EventTick
  (params (DeltaSeconds :type Float%20%28single-precision%29)))

(fn ConstructionScript)

(fn DecreaseHealth
  (params (Damage%20Taken :type Float%20%28double-precision%29))
  (bind _output_get (Variables|Health|SetCurrentHealth (Health|CalculateDecrementedHealth Damage%20Taken)))
  (if (<= _output_get 0.0)
    (return true)
    (else
      (return false))))

(fn CalculateDecrementedHealth
  (params (Damage%20Taken :type Float%20%28double-precision%29))
  (return (Math|Float|Clamp(Float) (- (Variables|Health|GetCurrentHealth) Damage%20Taken) 0.0 (Variables|Health|GetMaxHealth))))

(fn SetCurrentHealthtoMaxStart
  (Variables|Health|SetCurrentHealth (Variables|Health|GetMaxHealth)))

(fn SetCurrentStaminatoMaxonStart
  (Variables|Stamina|SetCurrentStamina (Variables|Stamina|GetMaxStamina)))

(fn IncreaseMaxHealth
  (params (MaxHealthGain :type Float%20%28double-precision%29))
  (bind _output_get (Variables|Health|SetMaxHealth (+ MaxHealthGain (Variables|Health|GetMaxHealth))))
  (return _output_get))

(fn DecreaseStamina
  (params (StaminaDepletion :type Float%20%28double-precision%29))
  (bind _output_get (Variables|Stamina|SetCurrentStamina (Stamina|CalculateDepletedStamina StaminaDepletion)))
  (if (<= _output_get 0.0)
    (return false)
    (else
      (return true))))

(fn CalculateDepletedStamina
  (params (StaminaDepletion :type Float%20%28double-precision%29))
  (return (Math|Float|Clamp(Float) (- (Variables|Stamina|GetCurrentStamina) StaminaDepletion) 0.0 (Variables|Stamina|GetMaxStamina))))

(fn IncreaseMaxStamina
  (params (MaxStaminaGain :type Float%20%28double-precision%29))
  (bind _output_get (Variables|Stamina|SetMaxStamina (+ MaxStaminaGain (Variables|Stamina|GetMaxStamina))))
  (return _output_get))